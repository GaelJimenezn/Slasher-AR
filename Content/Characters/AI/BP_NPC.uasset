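; NPC character that loses one life per damage event and is destroyed when its life runs out.
; Damage plays a hit reaction montage, updates a text display of remaining life, and grants one second of invulnerability.
; At zero life it calls a death montage and destroys the actor from the immediate output, without awaiting completion.
; Hits are reported as AI touch events, and Tick continually fixes walk speed.
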(event `self.ReceiveHit`
  (params (MyComp :type "PrimitiveComponent Object Reference") (Other :type "Actor Object Reference") (OtherComp :type "PrimitiveComponent Object Reference") (bSelfMoved :type Boolean) (HitLocation :type "Vector Structure") (HitNormal :type "Vector Structure") (NormalImpulse :type "Vector Structure") (Hit :type "HitResult Structure (by ref)"))
  (`AISense_Touch.ReportTouchEvent` self Other HitLocation))

(event `self.ReceiveTick`
  (params (DeltaSeconds :type "Float (single-precision)"))
  (set `CharacterMovementComponent.MaxWalkSpeed` 300.0 (`self.CharacterMovement`)))

(event `self.ReceiveAnyDamage`
  (params (Damage :type "Float (single-precision)") (DamageType :type "DamageType Object Reference") (InstigatedBy :type "Controller Object Reference") (DamageCauser :type "Actor Object Reference"))
  (if (not (`self.EsInvulnerable`))
    (set `self.EsInvulnerable` true)
    (bind _output_get (set `self.Vida` (- (`self.Vida`) 1)))
    (`|PlayMontage` null "/Game/Characters/AI/Anim/Standing_React_Small_From_Front_Montage.Standing_React_Small_From_Front_Montage"
      (:`then`
        (`TextRenderComponent.K2_SetText` (`self.TextRender`) (`KismetTextLibrary.Conv_IntToText` _output_get))
        (if (<= (`self.Vida`) 0)
          (`|PlayMontage` null "/Game/Characters/AI/Anim/Standing_React_Death_Backward_Montage.Standing_React_Death_Backward_Montage"
            (:`then`
              (`self.K2_DestroyActor`)))
          (else
            (`KismetSystemLibrary.Delay` 1.0)
            (set `self.EsInvulnerable` false)))))))

(fn `UserConstructionScript`)