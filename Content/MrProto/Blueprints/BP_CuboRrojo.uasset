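; BP_CuboRrojo is a damageable red cube actor in the MrProto prototype that shows its remaining health on a TextRender.
; Each AnyDamage event removes one point of Vida regardless of the damage amount, updates the text, and destroys the actor when health runs out.
; An EsInvulnerable flag with a one-second Delay gives a brief invulnerability window between hits.
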(event `self.ReceiveAnyDamage`
  (params (Damage :type "Float (single-precision)") (DamageType :type "DamageType Object Reference") (InstigatedBy :type "Controller Object Reference") (DamageCauser :type "Actor Object Reference"))
  (if (not (`self.EsInvulnerable`))
    (set `self.EsInvulnerable` true)
    (bind _output_get (set `self.Vida` (- (`self.Vida`) 1)))
    (`TextRenderComponent.K2_SetText` (`self.TextRender`) (`KismetTextLibrary.Conv_IntToText` _output_get))
    (if (<= (`self.Vida`) 0)
      (`self.K2_DestroyActor`)
      (else
        (`KismetSystemLibrary.Delay` 1.0)
        (set `self.EsInvulnerable` false)))))

(fn `UserConstructionScript`)